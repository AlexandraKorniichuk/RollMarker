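; Cleaner AI pawn that starts in the cleaners color and can trigger recoloring to the base color when it hits another RMAIPawn.
; On hit, it runs the parent logic, then passes the other pawn, cleaners color and base color to TryColorToTargetColor.
; The construction script creates the colored dynamic material, and a ColorMesh override zeroes its emissive when the applied color matches the target color.
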(event `self.ReceiveBeginPlay`)

(event `self.OnHit`
  (params (HitComponent :type "PrimitiveComponent Object Reference") (OtherActor :type "Actor Object Reference") (OtherComp :type "PrimitiveComponent Object Reference") (NormalImpulse :type "Vector Structure") (Hit :type "HitResult Structure (by ref)"))
  (bind _returnvalue (`RMSettings.Get`))
  (`parent.OnHit` HitComponent OtherActor OtherComp NormalImpulse Hit)
  (bind _asrmaipawn (cast `RMAIPawn` OtherActor))
  (`self.TryColorToTargetColor` _asrmaipawn (`RMSettings.CleanersColor` _returnvalue) (`RMSettings.BaseColor` _returnvalue)))

(event `self.ColorMesh`
  (params (Color :type "LinearColor Structure"))
  (`parent.ColorMesh` Color)
  (if (== Color (`RMSettings.TargetColor` (`RMSettings.Get`)))
    (`MaterialInstanceDynamic.SetScalarParameterValue` (`self.DynamicMaterial`) "Emissive" 0.0)))

(fn `UserConstructionScript`
  (`self.SetDynamicMaterial` (`RMSettings.CleanersColor` (`RMSettings.Get`))))